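; Player controller for a two-player, turn-based chat game between Host and Guest, linking the chat window to the game mode.
; After a short delay on BeginPlay it binds to WBP_ChatWindow's send-message event.
; Messages bound for the server reach BP_GameMode only when the saved UserID matches the GameState's TurnCount.
; It also pushes turn and score from GameState into the widget and prints broadcasts where it has authority.
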(event `self.ReceiveBeginPlay`
  ; Bind Event to Widget
  (if (not (`|EnumEquality` (`self.GetRemoteRole`) "ROLE_None"))
    (`KismetSystemLibrary.Delay` 0.5)
    (bind _foundwidgets (`WidgetBlueprintLibrary.GetAllWidgetsOfClass` "/Game/Widget/WBP_ChatWindow.WBP_ChatWindow_C"))
    (add `/Game/Widget/WBP_ChatWindow.CallSetMessageToUserController` (`|GetArrayItem` _foundwidgets) (`|CreateDelegate` :!event `OnSendMessageToServer`))
    (`self.UpdateTurnUI`)))

(event `OnSendMessageToServer`
  (params (Message :type String))
  (bind _userid (`self.UserID`))
  (bind _turncount (`/Game/BP/BP_GameStateBase.TurnCount` (cast `/Game/BP/BP_GameStateBase` (`GameplayStatics.GetGameState`) :!pure true)))
  ; Send Mesaage from client to server
  (bind _asbp_game_mode (cast `/Game/BP/BP_GameMode` (`GameplayStatics.GetGameMode`)))
  (if (and (`KismetStringLibrary.EqualEqual_StrStr` _userid "Host") (== _turncount 0))
    (`/Game/BP/BP_GameMode.GotMessageFromClient` _asbp_game_mode Message _userid)
    (elif (and (`KismetStringLibrary.EqualEqual_StrStr` _userid "Guest") (== _turncount 1))
      (`/Game/BP/BP_GameMode.GotMessageFromClient` _asbp_game_mode Message _userid))))

(event `GotBroadCast`
  (params (Message :type String))
  ; BroadCast Text from server
  (if (`self.HasAuthority`)
    (`KismetSystemLibrary.PrintString` Message)))

(event `OnLoginWithID`
  (params (UserID :type String))
  ; Login and Save Id
  (`self.OnUserLogin` UserID)
  (set `self.UserID` UserID))

(event `UpdateTurnUI`
  (bind _foundwidgets (`WidgetBlueprintLibrary.GetAllWidgetsOfClass` "/Game/Widget/WBP_ChatWindow.WBP_ChatWindow_C"))
  (switch `int` (`/Game/BP/BP_GameStateBase.TurnCount` (cast `/Game/BP/BP_GameStateBase` (`GameplayStatics.GetGameState`) :!pure true))
    (:`0`
      (bind _output (`|GetArrayItem` _foundwidgets))
      (`/Game/Widget/WBP_ChatWindow.SetTurn` _output "Host"))
    (:`1`
      (`/Game/Widget/WBP_ChatWindow.SetTurn` _output "Guest"))))

(event `UpdateScore`
  (bind _asbp_game_state_base (cast `/Game/BP/BP_GameStateBase` (`GameplayStatics.GetGameState`) :!pure true))
  (bind _foundwidgets (`WidgetBlueprintLibrary.GetAllWidgetsOfClass` "/Game/Widget/WBP_ChatWindow.WBP_ChatWindow_C"))
  (`/Game/Widget/WBP_ChatWindow.SetScore` (`|GetArrayItem` _foundwidgets) (`/Game/BP/BP_GameStateBase.HostScore` _asbp_game_state_base) (`/Game/BP/BP_GameStateBase.GuestScore` _asbp_game_state_base)))

(fn `UserConstructionScript`)