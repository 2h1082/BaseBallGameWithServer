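; Game state for a turn-based host-versus-guest match that pushes turn and score changes to player UI.
; RepNotify functions for TurnCount, HostScore and GuestScore each gather all PlayerControllers and cast them to BP_Controller.
; The turn notify calls UpdateTurnUI on each controller, while both score notifies call UpdateScore.
; The event graph and construction script hold no logic.
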(fn `OnRep_GuestScore`
  (bind _outactors (`GameplayStatics.GetAllActorsOfClass` "/Script/Engine.PlayerController"))
  (for _array_element _outactors
    (bind _asbp_controller (cast `/Game/BP/BP_Controller` _array_element))
    (`/Game/BP/BP_Controller.UpdateScore` _asbp_controller)))

(fn `OnRep_HostScore`
  (bind _outactors (`GameplayStatics.GetAllActorsOfClass` "/Script/Engine.PlayerController"))
  (for _array_element _outactors
    (bind _asbp_controller (cast `/Game/BP/BP_Controller` _array_element))
    (`/Game/BP/BP_Controller.UpdateScore` _asbp_controller)))

(fn `OnRep_TurnCount`
  (bind _outactors (`GameplayStatics.GetAllActorsOfClass` "/Script/Engine.PlayerController"))
  (for _array_element _outactors
    (bind _asbp_controller (cast `/Game/BP/BP_Controller` _array_element))
    (`/Game/BP/BP_Controller.UpdateTurnUI` _asbp_controller)))

(fn `UserConstructionScript`)