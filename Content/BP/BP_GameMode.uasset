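; Game mode for a two-player number-guessing game in which Host and Guest try to match a random unique three-digit number.
; On begin play it broadcasts the number to every BP_Controller, and later relays each client message the same way.
; Each message uses one of three chances, but only those containing "/" are judged for OUT, 3S or draw.
; Turn and scores go to BP_GameStateBase, and finished rounds reset after a delay.
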(event `self.ReceiveBeginPlay`
  (`KismetSystemLibrary.PrintString` "Game Start!!!")
  ; Generate Number
  (bind _returnvalue (`BaseBallGameFunction.GenerateUniqueThreeDigitNumber`))
  (bind _output_get (set `self.GeneratedNumber` _returnvalue))
  (bind _outactors (`GameplayStatics.GetAllActorsOfClass` "/Script/Engine.PlayerController"))
  (for _array_element _outactors
    (bind _asbp_controller (cast `/Game/BP/BP_Controller` _array_element))
    (`/Game/BP/BP_Controller.GotBroadCast` _asbp_controller (`KismetStringLibrary.Conv_IntToString` _output_get))))

(event `GotMessageFromClient`
  (params (Message :type String) (UserID :type String))
  (bind _user_id (`self.User ID`))
  (bind _asbp_game_state_base (cast `/Game/BP/BP_GameStateBase` (`GameplayStatics.GetGameState`) :!pure true))
  (set `self.User ID` UserID)
  (`|ExecutionSequence`
    (:`then_0`
      (bind _outactors (`GameplayStatics.GetAllActorsOfClass` "/Script/Engine.PlayerController"))
      (for _array_element _outactors
        (bind _asbp_controller (cast `/Game/BP/BP_Controller` _array_element))
        (`/Game/BP/BP_Controller.GotBroadCast` _asbp_controller (`KismetStringLibrary.Concat_StrStr` (`self.User ID`) ":" Message))))
    (:`then_1`
      (switch `string` (`self.User ID`)
        (:`Host`
          (if (< (`self.HostChance`) 3)
            (set `self.HostChance` (+ (`self.HostChance`) 1))
            (if (`KismetStringLibrary.Contains` Message "/") :!label _label
              (bind _returnvalue (`BaseBallGameFunction.ResultJudgment` (`self.GeneratedNumber`) Message))
              (bind _output_get (set `self.TurnCount` (mod (+ (`self.TurnCount`) 1) 2)))
              (bind _asbp_game_state_base_2 (cast `/Game/BP/BP_GameStateBase` (`GameplayStatics.GetGameState`)))
              (set `/Game/BP/BP_GameStateBase.TurnCount` _output_get _asbp_game_state_base_2)
              (`KismetSystemLibrary.PrintString` _returnvalue)
              (if (`KismetStringLibrary.EqualEqual_StrStr` _returnvalue "OUT")
                (switch `string` (`self.User ID`)
                  (:`Host`
                    (`KismetSystemLibrary.PrintString` "Guest Win!")
                    (bind _output_get_2 (set `self.GuestWinCount` (+ (`self.GuestWinCount`) 1) :!label _label_2))
                    (set `/Game/BP/BP_GameStateBase.GuestScore` _output_get_2 _asbp_game_state_base))
                  (:`Guest`
                    (`KismetSystemLibrary.PrintString` "Host Win!")
                    (bind _output_get_3 (set `self.HostWinCount` (+ (`self.HostWinCount`) 1) :!label _label_3))
                    (set `/Game/BP/BP_GameStateBase.HostScore` _output_get_3 _asbp_game_state_base)))
                (`KismetSystemLibrary.PrintString` "Game End!!!" :!label _label_4)
                (`KismetSystemLibrary.Delay` 3.0)
                (`self.ResetGame`)
                (elif (and (>= (`self.HostChance`) 3) (>= (`self.GuestChance`) 3))
                  (`KismetSystemLibrary.PrintString` "Draw!")
                  (goto _label_4)
                  (elif (`KismetStringLibrary.Contains` _returnvalue "3S")
                    (`KismetSystemLibrary.PrintString` (`KismetStringLibrary.Concat_StrStr` _user_id " Win!"))
                    (if (`KismetStringLibrary.EqualEqual_StrStr` _user_id "Host")
                      (goto _label_3)
                      (else
                        (goto _label_2))))))
              (else
                (`KismetSystemLibrary.PrintString` "Please enter '/' first!")))
            (else
              (`KismetSystemLibrary.PrintString` "No Chance (Host)"))))
        (:`Guest`
          (if (< (`self.GuestChance`) 3)
            (set `self.GuestChance` (+ (`self.GuestChance`) 1))
            (goto _label)
            (else
              (`KismetSystemLibrary.PrintString` "No Chance (Guest"))))))))

(event `ResetGame`
  (`KismetSystemLibrary.PrintString` "Game Start!!!")
  (bind _returnvalue (`BaseBallGameFunction.GenerateUniqueThreeDigitNumber`))
  (set `self.GeneratedNumber` _returnvalue)
  (set `self.HostChance` 0)
  (set `self.GuestChance` 0)
  (bind _output_get (set `self.TurnCount` 0))
  (bind _asbp_game_state_base (cast `/Game/BP/BP_GameStateBase` (`GameplayStatics.GetGameState`)))
  (set `/Game/BP/BP_GameStateBase.TurnCount` _output_get _asbp_game_state_base))

(fn `UserConstructionScript`)